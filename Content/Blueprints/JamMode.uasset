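; JamMode is the game flow Blueprint for a jam game with a ghost character, running title screen, play and win screen.
; BeginPlay creates the title, HUD and end widgets, then Reset clears state flags, resets the Neighborhood and ghost, and destroys LooseItems.
; Begin switches to play UI and input.
; NotifyWin starts a one-second timer for ShowWin, which plays a sound and shows the end screen with UI-only input.
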(event `self.ReceiveBeginPlay`
  (bind _returnvalue (`GameplayStatics.GetPlayerController` 0))
  (`|ExecutionSequence`
    (:`then_0`
      (`WidgetBlueprintLibrary.SetFocusToGameViewport`)
      (`WidgetBlueprintLibrary.SetInputMode_UIOnlyEx` (`GameplayStatics.GetPlayerController` 0) null "LockOnCapture"))
    (:`then_1`
      (bind _returnvalue_2 (`|CreateWidget` "/Game/Blueprints/UI/TitleScreen.TitleScreen_C" _returnvalue))
      (bind _output_get (set `self.TitleScreenWidget` _returnvalue_2))
      (`UserWidget.AddToViewport` _output_get 0)
      (bind _returnvalue_3 (`|CreateWidget` "/Game/Blueprints/UI/JamHUD.JamHUD_C" _returnvalue))
      (bind _output_get_2 (set `self.HUDWidget` _returnvalue_3))
      (`UserWidget.AddToViewport` _output_get_2 0)
      (bind _returnvalue_4 (`|CreateWidget` "/Game/Blueprints/UI/EndScreen.EndScreen_C" _returnvalue))
      (bind _output_get_3 (set `self.EndScreenWidget` _returnvalue_4))
      (`UserWidget.AddToViewport` _output_get_3 0)
      (`Widget.SetVisibility` _output_get_3 "Hidden"))
    (:`then_2`
      (`self.Reset`))))

(fn `Begin`
  (set `self.Playing` true)
  (`Widget.SetVisibility` (`self.TitleScreenWidget`) "Hidden")
  (`Widget.SetVisibility` (`self.HUDWidget`) "Visible")
  (`Widget.SetVisibility` (`self.EndScreenWidget`) "Hidden")
  (`WidgetBlueprintLibrary.SetInputMode_GameAndUIEx` (`GameplayStatics.GetPlayerController` 0) null "LockOnCapture"))

(fn `NotifyWin`
  (`KismetSystemLibrary.K2_SetTimer` null "ShowWin" 1.0))

(fn `Reset`
  (`|ExecutionSequence`
    (:`then_0`
      (set `self.Playing` false)
      (set `self.GameOver` false))
    (:`then_1`
      (bind _outactors (`GameplayStatics.GetAllActorsOfClass` "/Game/Blueprints/Neighborhood.Neighborhood_C"))
      (`/Game/Blueprints/Neighborhood.Reset` (`|GetArrayItem` _outactors)))
    (:`then_2`
      (bind _outactors_2 (`GameplayStatics.GetAllActorsOfClass` "/Game/Blueprints/LooseItem.LooseItem_C"))
      (for _array_element _outactors_2
        (`self.K2_DestroyActor` _array_element)))
    (:`then_3`
      (bind _asghost_character (cast `/Game/Blueprints/GhostCharacter` (`GameplayStatics.GetPlayerPawn` 0)))
      (`/Game/Blueprints/GhostCharacter.Reset` _asghost_character))))

(fn `ShowWin`
  (bind _endscreenwidget (`self.EndScreenWidget`))
  (`GameplayStatics.PlaySoundAtLocation` "/Game/Sound/Win.Win" (`self.K2_GetActorLocation` (`GameplayStatics.GetPlayerPawn` 0)) (struct) 1.0 1.0 0.0 null null null)
  (`Widget.SetVisibility` _endscreenwidget "Visible")
  (`WidgetBlueprintLibrary.SetInputMode_UIOnlyEx` (`GameplayStatics.GetPlayerController` 0) _endscreenwidget))

(fn `UserConstructionScript`)