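; Beam effect actor that stretches a mesh and a Niagara system between two points.
; Place aims the actor from start to end, scales mesh Z by distance, matches the dynamic material's LengthScale and sets the Niagara endpoints.
; Appear plays a timeline that animates mesh thickness, with event tracks revealing the mesh and activating the particles.
; A disappear timeline has a mesh-hiding event, but nothing here plays it.
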(event `self.ReceiveBeginPlay`
  (bind _returnvalue (`KismetMaterialLibrary.CreateDynamicMaterialInstance` "/Game/Materials/MeshBeamMaterial.MeshBeamMaterial"))
  (bind _output_get (set `self.BeamMaterialInstance` _returnvalue))
  (`PrimitiveComponent.SetMaterial` (`self.MainBeamMesh`) 0 _output_get))

(fn `Appear`
  (`TimelineComponent.PlayFromStart` (`self.AppearTimeline`)))

(fn `Place`
  (params (Start :type "Vector Structure") (End :type "Vector Structure"))
  (bind _mainbeammesh (`self.MainBeamMesh`))
  (bind _beamsystem (`self.BeamSystem`))
  (bind _returnvalue (/ (`KismetMathLibrary.Vector_Distance` Start End) 100.0))
  (bind (_relativescale3d_x _relativescale3d_y) (`KismetMathLibrary.BreakVector` (`SceneComponent.RelativeScale3D` _mainbeammesh)))
  (`self.K2_SetActorTransform` (`KismetMathLibrary.MakeTransform` Start (`KismetMathLibrary.FindLookAtRotation` Start End)))
  (`SceneComponent.SetRelativeScale3D` _mainbeammesh (`KismetMathLibrary.MakeVector` _relativescale3d_x _relativescale3d_y _returnvalue))
  (`MaterialInstanceDynamic.SetScalarParameterValue` (`self.BeamMaterialInstance`) "LengthScale" _returnvalue)
  (`NiagaraComponent.SetNiagaraVariableVec3` _beamsystem "User.StartPoint" Start)
  (`NiagaraComponent.SetNiagaraVariableVec3` _beamsystem "User.EndPoint" End))

(fn `UserConstructionScript`)