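; House actor with a dig spot that can hold one buried inventory item.
; Construction randomizes the DigArea position, and BeginPlay may bury a random item based on ItemProbability.
; Functions query, remove, bury and reserve the spot with a pending flag, while the HoleIndicator's Z scale reflects whether it is filled.
; GhostCharacter overlap events are stubs with no effect.
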(event `self.ReceiveBeginPlay`
  (if (< (`KismetMathLibrary.RandomFloat`) (`self.ItemProbability`))
    (`self.BuryItem` (cast `/Game/Blueprints/InventoryItem` (`KismetMathLibrary.Conv_IntToByte` (`KismetMathLibrary.RandomIntegerInRange` 0 (- (enumcount `/Game/Blueprints/InventoryItem`) 1)))))))

(event `self.ReceiveActorBeginOverlap`
  (params (OtherActor :type "Actor Object Reference"))
  (cast `/Game/Blueprints/GhostCharacter` OtherActor)
  (if (`self.HasBuriedItem`)
    _))

(event `self.ReceiveActorEndOverlap`
  (params (OtherActor :type "Actor Object Reference"))
  (cast `/Game/Blueprints/GhostCharacter` OtherActor))

(fn `BuryItem`
  (params (Item :type "/Game/Blueprints/InventoryItem Enum" :default "NewEnumerator0"))
  (set `self.BuriedItem` Item)
  (`self.SetHasBuriedItem` true))

(fn `CanBuryHere`
  (returns (Can :type Boolean))
  (return (not (or (`self.HasBuriedItem`) (`self.HasPendingBurial`)))))

(fn `GetBuriedItem`
  (returns (Has :type Boolean) (Item :type "/Game/Blueprints/InventoryItem Enum"))
  (return (`self.HasBuriedItem`) (`self.BuriedItem`)))

(fn `RegisterIntentToBury`
  (set `self.HasPendingBurial` true))

(fn `RemoveBuriedItem`
  (`self.SetHasBuriedItem` false))

(fn `SetHasBuriedItem`
  (params (Has :type Boolean))
  (bind _holeindicator (`self.HoleIndicator`))
  (bind _returnvalue (`SceneComponent.GetRelativeTransform` _holeindicator))
  (bind _output_get (set `self.HasBuriedItem` Has))
  (set `self.HasPendingBurial` false)
  (`SceneComponent.SetRelativeScale3D` _holeindicator (`KismetMathLibrary.MakeVector` (.x (.scale _returnvalue)) (.y (.scale _returnvalue)) (`KismetMathLibrary.SelectFloat` 0.5 0.15 _output_get))))

(fn `UserConstructionScript`
  (bind _digarea (`self.DigArea`))
  (bind (_relativelocation_x _relativelocation_y _relativelocation_z) (`KismetMathLibrary.BreakVector` (`SceneComponent.RelativeLocation` _digarea)))
  (`SceneComponent.K2_SetRelativeLocation` _digarea (`KismetMathLibrary.MakeVector` (`KismetMathLibrary.RandomFloatInRange` -350.0 350.0) (`KismetMathLibrary.RandomFloatInRange` 200.0 480.0) _relativelocation_z) false false))