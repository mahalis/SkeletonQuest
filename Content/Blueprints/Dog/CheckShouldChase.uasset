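; Behavior tree service for the Dog AI that decides whether it should chase the player's ghost character.
; On each AI tick it casts the player pawn to GhostCharacter, then checks that the ghost has any item and is within a fixed range of the dog.
; When both hold it writes the player pawn to the target blackboard key, otherwise it clears that key.
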(event `self.ReceiveTickAI`
  (params (OwnerController :type "AIController Object Reference") (ControlledPawn :type "Pawn Object Reference") (DeltaSeconds :type "Float (single-precision)"))
  (bind _returnvalue (`GameplayStatics.GetPlayerPawn` 0))
  (bind _targetplayerkey (`self.TargetPlayerKey`))
  (bind _asghost_character (cast `/Game/Blueprints/GhostCharacter` _returnvalue))
  (if (and (`/Game/Blueprints/GhostCharacter.HasAnyItem` _asghost_character) (< (`KismetMathLibrary.Vector_Distance` (`Actor.K2_GetActorLocation` ControlledPawn) (`Actor.K2_GetActorLocation` _returnvalue)) 600.0))
    (`BTFunctionLibrary.SetBlackboardValueAsObject` _targetplayerkey _returnvalue)
    (else
      (`BTFunctionLibrary.ClearBlackboardValue` _targetplayerkey))))