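; Behavior tree task that has an AI-controlled Dog bury its carried item at a House.
; On execute, it reads the House from a blackboard key, passes the Dog's item to BuryItem, then removes the item from the Dog.
; It finishes successfully even with no item, a case marked as unreachable, but never finishes if either cast fails.
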(event `self.ReceiveExecuteAI`
  (params (OwnerController :type "AIController Object Reference") (ControlledPawn :type "Pawn Object Reference"))
  (bind _asdog (cast `/Game/Blueprints/Dog/Dog` ControlledPawn))
  (bind _ashouse (cast `/Game/Blueprints/House` (`BTFunctionLibrary.GetBlackboardValueAsActor` (`self.HouseKey`))))
  (if (`/Game/Blueprints/Dog/Dog.HasItem` _asdog)
    (`/Game/Blueprints/House.BuryItem` _ashouse (`/Game/Blueprints/Dog/Dog.Item` _asdog))
    (`/Game/Blueprints/Dog/Dog.RemoveItem` _asdog)
    (`self.FinishExecute` true)
    (else
      (`self.FinishExecute` true) ; shouldn't be reachable, we should never try to bury without an item to bury
    )))