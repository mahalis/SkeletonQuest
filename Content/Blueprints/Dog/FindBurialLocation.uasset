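; Behavior tree task for the dog AI that picks a random House to bury at.
; It shuffles all House actors, takes the first that allows burying and registers the intent to bury on it.
; That house and its DigArea world location go into blackboard keys, and the task succeeds only if a house is found.
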(event `self.ReceiveExecuteAI`
  (params (OwnerController :type "AIController Object Reference") (ControlledPawn :type "Pawn Object Reference"))
  (bind _found (`self.Find`))
  (`self.FinishExecute` _found))

(fn `Find`
  (returns (Found :type Boolean))
  (locals (ShuffledHouses :type "Array of /Game/Blueprints/House Object Reference"))
  (bind _outactors (`GameplayStatics.GetAllActorsOfClass` "/Game/Blueprints/House.House_C"))
  (bind _output_get (set `local.ShuffledHouses` _outactors))
  (`KismetArrayLibrary.Array_Shuffle` _output_get)
  (for _array_element (`local.ShuffledHouses`)
    (if (`/Game/Blueprints/House.CanBuryHere` _array_element)
      (`/Game/Blueprints/House.RegisterIntentToBury` _array_element)
      (`BTFunctionLibrary.SetBlackboardValueAsObject` (`self.HouseKey`) _array_element)
      (`BTFunctionLibrary.SetBlackboardValueAsVector` (`self.LocationKey`) (`SceneComponent.K2_GetComponentLocation` (`/Game/Blueprints/House.DigArea` _array_element)))
      (return true)))
  (return false))