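; AttemptSteal is a behavior tree task in which the Dog tries to steal an item from the player's GhostCharacter.
; On execute it casts the player pawn and controlled pawn, asks the ghost to remove any item, and stores the result in the dog's HasItem and Item.
; The task finishes with the removal's success and prints the stolen item's name when it succeeds.
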(event `self.ReceiveExecuteAI`
  (params (OwnerController :type "AIController Object Reference") (ControlledPawn :type "Pawn Object Reference"))
  (bind _asghost_character (cast `/Game/Blueprints/GhostCharacter` (`GameplayStatics.GetPlayerPawn` 0)))
  (bind _asdog (cast `/Game/Blueprints/Dog/Dog` ControlledPawn))
  (bind (_item _success) (`/Game/Blueprints/GhostCharacter.RemoveAnyItem` _asghost_character))
  (set `/Game/Blueprints/Dog/Dog.HasItem` _success _asdog)
  (bind _output_get (set `/Game/Blueprints/Dog/Dog.Item` _item _asdog))
  (`self.FinishExecute` _success)
  (if _success
    (`KismetSystemLibrary.PrintString` (`KismetStringLibrary.Concat_StrStr` "stole a " (`|GetEnumeratorNameAsString` _output_get)))))