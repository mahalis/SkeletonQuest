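; Behavior tree node that decides whether a Dog AI can keep chasing, based on its home territory.
; Each AI tick it writes the within-territory Blackboard bool, true only while the target object is valid and either player pawn 0 or the dog is inside the chase radius around the home's TerritoryOrigin.
; The distance check uses the first player's pawn rather than the Blackboard target's location.
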(event `self.ReceiveTickAI`
  (params (OwnerController :type "AIController Object Reference") (ControlledPawn :type "Pawn Object Reference") (DeltaSeconds :type "Float (single-precision)"))
  (bind _validchaseradius (`self.ValidChaseRadius`))
  (bind _asdog (cast `/Game/Blueprints/Dog/Dog` ControlledPawn))
  (bind _returnvalue (`SceneComponent.K2_GetComponentLocation` (`/Game/Blueprints/House.TerritoryOrigin` (`/Game/Blueprints/Dog/Dog.Home` _asdog))))
  (`BTFunctionLibrary.SetBlackboardValueAsBool` (`self.WithinTerritoryKey`) (and (`KismetSystemLibrary.IsValid` (`BTFunctionLibrary.GetBlackboardValueAsObject` (`self.TargetKey`))) (or (< (`KismetMathLibrary.Vector_Distance` (`Actor.K2_GetActorLocation` (`GameplayStatics.GetPlayerPawn` 0)) _returnvalue) _validchaseradius) (< (`KismetMathLibrary.Vector_Distance` (`Actor.K2_GetActorLocation` ControlledPawn) _returnvalue) _validchaseradius)))))