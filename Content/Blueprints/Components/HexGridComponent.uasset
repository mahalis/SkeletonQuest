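; Component that converts between cell coordinates and 2D positions on a flat-topped hex grid with staggered columns.
; MakeMetrics derives column and row spacing from Radius, and both conversion functions use it, shifting alternate columns by half a row.
; CellFromPosition floors the position to a rectangular tile, then tests the slanted edge to choose that cell or one in the previous column, without branching.
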(event `self.ReceiveBeginPlay`)

(fn `CellFromPosition`
  (params (PositionX :type "Float (double-precision)") (PositionY :type "Float (double-precision)"))
  (returns (X :type Integer) (Y :type Integer))
  (locals (TileX :type "Float (double-precision)") (TileY :type "Float (double-precision)") (TileColumn :type Integer) (TileRow :type Integer) (InMainTileArea :type Boolean) (SpacingX :type "Float (double-precision)") (SpacingY :type "Float (double-precision)"))
  (bind _tilecolumn (`local.TileColumn`))
  (bind _tilerow (`local.TileRow`))
  (bind _returnvalue (- PositionY (* (mod (`local.TileColumn`) 2) (* (`local.SpacingY`) 0.5))))
  (bind (_horizontalspacing _verticalspacing) (`self.MakeMetrics`))
  (set `local.SpacingX` _horizontalspacing)
  (set `local.SpacingY` _verticalspacing)
  (set `local.TileColumn` (`KismetMathLibrary.FFloor` (/ PositionX _horizontalspacing)))
  (set `local.TileRow` (`KismetMathLibrary.FFloor` (/ _returnvalue (`local.SpacingY`))))
  ;[1 1 1] tile-local coordinate
  (bind _output_get (set `local.TileX` (- PositionX (* (`local.TileColumn`) (`local.SpacingX`)))))
  (bind _output_get_2 (set `local.TileY` (- _returnvalue (* (`local.TileRow`) (`local.SpacingY`)))))
  (bind _output_get_3 (set `local.InMainTileArea` (> _output_get (* (`self.Radius`) (`KismetMathLibrary.Abs` (- 0.5 (/ _output_get_2 _verticalspacing)))))))
  (return (`KismetMathLibrary.SelectInt` _tilecolumn (- _tilecolumn 1) _output_get_3) (`KismetMathLibrary.SelectInt` _tilerow (+ _tilerow (`KismetMathLibrary.SelectInt` 0 1 (> (`local.TileY`) (* (`local.SpacingY`) 0.5)))) _output_get_3)))

(fn `MakeMetrics`
  (returns (HorizontalSpacing :type "Float (double-precision)") (VerticalSpacing :type "Float (double-precision)"))
  (bind _radius (`self.Radius`))
  (return (* _radius 1.5) (* _radius 1.732051)))

(fn `PositionFromCell`
  (params (CellX :type Integer) (CellY :type Integer))
  (returns (X :type "Float (double-precision)") (Y :type "Float (double-precision)"))
  (bind (_horizontalspacing _verticalspacing) (`self.MakeMetrics`))
  (return (* CellX _horizontalspacing) (+ (* CellY _verticalspacing) (* (mod CellX 2) (* _verticalspacing 0.5)))))