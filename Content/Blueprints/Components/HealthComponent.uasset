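; Health component that tracks Health and an IsAlive flag, with TakeDamage and Heal functions that act only while alive.
; TakeDamage's check is inverted: damage leaving Health above zero clears IsAlive, fires Died, zeroes Health and returns true, while lethal damage only subtracts.
; That subtract branch and Heal, which adds without an upper clamp, timestamp the change in LastHealthChangeTime.
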(fn `Heal`
  (params (Amount :type "Float (double-precision)"))
  (if (`self.IsAlive`)
    (set `self.Health` (+ (`self.Health`) Amount))
    (set `self.LastHealthChangeTime` (`KismetSystemLibrary.GetGameTimeInSeconds`))))

(fn `TakeDamage`
  (params (Amount :type "Float (double-precision)"))
  (returns (Died :type Boolean))
  (bind _returnvalue (- (`self.Health`) Amount))
  (if (`self.IsAlive`)
    (if (> _returnvalue 0.0)
      (set `self.IsAlive` false)
      (`self.Died`)
      (set `self.Health` 0.0)
      (return true)
      (else
        (set `self.Health` _returnvalue)
        (set `self.LastHealthChangeTime` (`KismetSystemLibrary.GetGameTimeInSeconds`))
        (return false)))))