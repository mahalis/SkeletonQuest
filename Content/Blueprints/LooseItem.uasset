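; LooseItem is an actor representing a loose body part (skull, torso, arm or leg) with a pickup area.
; ApplyMesh runs on BeginPlay and SetItem, selecting the static mesh for RepresentedItem, with left and right limbs sharing a mesh.
; It also moves PickupArea to the center of that mesh's bounding box.
; GetItem exposes the represented part; no overlap or pickup logic runs here.
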(event `self.ReceiveBeginPlay`
  (`self.ApplyMesh`))

(fn `ApplyMesh`
  (bind _returnvalue (select `/Game/Blueprints/InventoryItem` (`self.RepresentedItem`) :`NewEnumerator0` "/Game/Meshes/skull.Skull" :`NewEnumerator1` "/Game/Meshes/Torso.Torso" :`NewEnumerator2` "/Game/Meshes/armleg.ArmLeg" :`NewEnumerator3` "/Game/Meshes/armleg.ArmLeg" :`NewEnumerator4` "/Game/Meshes/Leg.Leg" :`NewEnumerator5` "/Game/Meshes/Leg.Leg" :!type "StaticMesh Object Reference"))
  (bind (_returnvalue_min _returnvalue_max) (break `Box` (`StaticMesh.GetBoundingBox` _returnvalue)))
  (`StaticMeshComponent.SetStaticMesh` (`self.Mesh`) _returnvalue)
  (`SceneComponent.K2_SetRelativeLocation` (`self.PickupArea`) (`KismetMathLibrary.VLerp` _returnvalue_min _returnvalue_max 0.5) false false))

(fn `GetItem`
  (returns (Item :type "/Game/Blueprints/InventoryItem Enum"))
  (return (`self.RepresentedItem`)))

(fn `SetItem`
  (params (Item :type "/Game/Blueprints/InventoryItem Enum" :default "NewEnumerator0"))
  (set `self.RepresentedItem` Item)
  (`self.ApplyMesh`))

(fn `UserConstructionScript`)