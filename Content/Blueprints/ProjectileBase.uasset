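; Base projectile actor that, on hit, stops its movement, pushes physics objects and removes itself.
; A hit hides the mesh, deactivates the trail and disables collision, then a timer destroys the actor after a short delay.
; For a valid hit actor with a simulating component, it applies an impulse from velocity and an impact multiplier, read after movement has stopped.
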(event `self.ReceiveHit`
  (params (MyComp :type "PrimitiveComponent Object Reference") (Other :type "Actor Object Reference") (OtherComp :type "PrimitiveComponent Object Reference") (bSelfMoved :type Boolean) (HitLocation :type "Vector Structure") (HitNormal :type "Vector Structure") (NormalImpulse :type "Vector Structure") (Hit :type "HitResult Structure (by ref)"))
  (`self.PrepareToSelfDestruct`)
  (`ProjectileMovementComponent.StopSimulating` (`self.ProjectileMovement`) Hit)
  (`/Engine/EditorBlueprintResources/StandardMacros.IsValid` Other
    (:`Is Valid`
      (`self.ApplyImpactForce` OtherComp))))

(fn `ApplyImpactForce`
  (params (OtherComponent :type "PrimitiveComponent Object Reference"))
  (if (`SceneComponent.IsSimulatingPhysics` OtherComponent "None")
    (`PrimitiveComponent.AddImpulseAtLocation` OtherComponent (* (`self.GetVelocity`) (`self.ImpactForceMultiplier`)) (`self.K2_GetActorLocation`) "None")))

(fn `FinishSelfDestructing`
  (`self.K2_DestroyActor`))

(fn `PrepareToSelfDestruct`
  (`SceneComponent.SetVisibility` (`self.Mesh`) false false)
  (`ActorComponent.Deactivate` (`self.Trail`))
  (`PrimitiveComponent.SetCollisionEnabled` (`self.Collision`) "NoCollision")
  (`KismetSystemLibrary.K2_SetTimer` null "FinishSelfDestructing" 1.0))

(fn `UserConstructionScript`)