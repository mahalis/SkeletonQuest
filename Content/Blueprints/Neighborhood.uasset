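; Neighborhood actor that spawns a grid of House actors when play begins.
; MakeHouses loops over Width by Depth, placing each house at HouseSpacing intervals, centered on the world origin rather than on the actor's own location.
; Each house spawns regardless of collision and is stored in the Houses array.
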(event `self.ReceiveBeginPlay`
  (`self.MakeHouses`))

(fn `MakeHouses`
  (bind _housespacing (`self.HouseSpacing`))
  (for _index (range 1 (+ (`self.Width`) 1))
    (for _index_2 (range 1 (+ (`self.Depth`) 1))
      (bind (_returnvalue_x _returnvalue_y) (`KismetMathLibrary.BreakVector2D` (+ (* (* (`self.HouseSpacing`) (`KismetMathLibrary.MakeVector2D` (`KismetMathLibrary.Conv_IntToDouble` (`self.Width`)) (`KismetMathLibrary.Conv_IntToDouble` (`self.Depth`)))) -0.5) (* _housespacing (`KismetMathLibrary.MakeVector2D` (`KismetMathLibrary.Conv_IntToDouble` (- _index 1)) (`KismetMathLibrary.Conv_IntToDouble` (- _index_2 1)))) (* _housespacing 0.5))))
      (bind _returnvalue (`|SpawnActorFromClass` "/Game/Blueprints/House.House_C" (`KismetMathLibrary.MakeTransform` (`KismetMathLibrary.MakeVector` _returnvalue_x _returnvalue_y)) "AlwaysSpawn" "OverrideRootScale" null null))
      (`KismetArrayLibrary.Array_Add` (`self.Houses`) _returnvalue))))

(fn `UserConstructionScript`)